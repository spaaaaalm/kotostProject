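; AI controller for BP_Enemy that chases and attacks the first player character, tuned by the enemy's EnemyConfig.
; Tick runs hand-rolled perception (range with lose-sight hysteresis, view cone, line of sight, memory timer) feeding an Idle/Chase/Attack state machine.
; Chase turns toward the player and throttles repathing; Attack applies cooldown-gated damage through BPI_Damageable.
; The enemy's death and revive events stop and restart the behavior.
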(event Custom|HandleEnemyDied
  (Variables|Default|SetbBehaviorStopped true)
  (Variables|Default|SetAIState "NewEnumerator0")
  (Variables|Default|SetbHasTarget false)
  (Variables|Default|SetbSeesTarget false)
  (Variables|Default|SetLostSightTimer 0.0)
  (AI|Navigation|StopMovement))

(event Custom|HandleEnemyRevived
  (Variables|Default|SetbBehaviorStopped false)
  (Variables|Default|SetAIState "NewEnumerator0")
  (Variables|Default|SetbHasTarget false)
  (Variables|Default|SetbSeesTarget false)
  (Variables|Default|SetLostSightTimer 0.0)
  (Variables|Default|SetLastAttackTime -1e+03)
  (AI|Navigation|StopMovement))

(event EventPossess
  (params (PossessedPawn :type Pawn%20Object%20Reference))
  (bind _asbp_enemy (Utilities|Casting|CastToBP_Enemy PossessedPawn))
  (Variables|Default|SetEnemyCharacter _asbp_enemy)
  (Variables|Default|SetEnemyConfig (Variables|/Game/Enemies/BP_Enemy.BP_Enemy_C|GetEnemyConfig _asbp_enemy))
  (EventDispatchers|BindEventtoOnEnemyDied _asbp_enemy (EventDispatchers|CreateEvent :!event Custom|HandleEnemyDied))
  (EventDispatchers|BindEventtoOnEnemyRevived _asbp_enemy (EventDispatchers|CreateEvent :!event Custom|HandleEnemyRevived))
  (Variables|Default|SetPlayerTarget (Game|GetPlayerCharacter 0))
  (Variables|Default|SetAIState "NewEnumerator0")
  (Variables|Default|SetbBehaviorStopped false)
  (Variables|Default|SetbHasTarget false)
  (Variables|Default|SetbSeesTarget false)
  (Variables|Default|SetLostSightTimer 0.0)
  (Variables|Default|SetLastAttackTime -1e+03)
  (Variables|Default|SetLastMoveRequestTime -1e+03))

(event EventTick
  (params (DeltaSeconds :type Float%20%28single-precision%29))
  (bind _enemyconfig (Variables|Default|GetEnemyConfig))
  (bind _bhastarget (Variables|Default|GetbHasTarget))
  (bind _bseestarget (Variables|Default|GetbSeesTarget))
  (bind _targetdistance (Variables|Default|GetTargetDistance))
  (bind _attackrange (Variables|/Game/Data/BP_EnemyConfig.BP_EnemyConfig_C|GetAttackRange _enemyconfig))
  (if (not (Variables|Default|GetbBehaviorStopped))
    (if (and (Utilities|IsValid _enemyconfig) (Utilities|IsValid (Variables|Default|GetEnemyCharacter)))
      (CallFunction|UpdatePerception DeltaSeconds)
      (switch Utilities|FlowControl|Switch|SwitchonE_EnemyAIState (Variables|Default|GetAIState)
        (:NewEnumerator0
          (if _bhastarget
            (CallFunction|EnterState "NewEnumerator1")))
        (:NewEnumerator1
          (if _bhastarget
            (if (<= _targetdistance _attackrange)
              (CallFunction|EnterState "NewEnumerator2")
              (else
                (CallFunction|FacePlayerTarget DeltaSeconds)
                (if _bseestarget
                  (if (and (!= (Class|AIController|GetMoveStatus) 3) (>= (- (Utilities|Time|GetGameTimeinSeconds) (Variables|Default|GetLastMoveRequestTime)) (Variables|/Game/Data/BP_EnemyConfig.BP_EnemyConfig_C|GetChaseRepathInterval _enemyconfig)))
                    (AI|Navigation|MovetoActor (Variables|Default|GetPlayerTarget) (* _attackrange 0.8) true true true 0)
                    (Variables|Default|SetLastMoveRequestTime (Utilities|Time|GetGameTimeinSeconds)))
                  (else
                    (AI|Navigation|StopMovement)))))
            (else
              (CallFunction|EnterState "NewEnumerator0"))))
        (:NewEnumerator2
          (if _bhastarget
            (if (> _targetdistance _attackrange)
              (CallFunction|EnterState "NewEnumerator1")
              (else
                (CallFunction|FacePlayerTarget DeltaSeconds)
                (if _bseestarget
                  (CallFunction|TryAttack))))
            (else
              (CallFunction|EnterState "NewEnumerator0"))))))))

(fn ConstructionScript)

(fn UpdatePerception
  (params (DeltaSeconds :type Float%20%28single-precision%29))
  (bind _enemycharacter (Variables|Default|GetEnemyCharacter))
  (bind _enemyconfig (Variables|Default|GetEnemyConfig))
  (if (Utilities|IsValid _enemycharacter)
    (if (Utilities|IsValid (Variables|Default|GetPlayerTarget))
      (Variables|Default|SetTargetDistance (Math|Vector|VectorLength (- (Transformation|GetActorLocation (Variables|Default|GetPlayerTarget)) (Transformation|GetActorLocation _enemycharacter))))
      (Variables|Default|SetbSeesTarget (and (and (and (<= (Variables|Default|GetTargetDistance) (Math|Float|SelectFloat (Variables|/Game/Data/BP_EnemyConfig.BP_EnemyConfig_C|GetLoseSightRadius _enemyconfig) (Variables|/Game/Data/BP_EnemyConfig.BP_EnemyConfig_C|GetSightRadius _enemyconfig) (Variables|Default|GetbHasTarget))) (<= (Class|KismetMathLibrary|DegAcos (Math|Vector|DotProduct (Math|Vector|Normalize (- (Transformation|GetActorLocation (Variables|Default|GetPlayerTarget)) (Transformation|GetActorLocation _enemycharacter))) (Transformation|GetActorForwardVector _enemycharacter))) (Variables|/Game/Data/BP_EnemyConfig.BP_EnemyConfig_C|GetPeripheralVisionAngleDegrees _enemyconfig))) (Utilities|IsValid (Variables|Default|GetPlayerTarget))) (Controller|LineOfSightTo (Variables|Default|GetPlayerTarget) "0, 0, 0" false)))
      (if (Variables|Default|GetbSeesTarget)
        (Variables|Default|SetbHasTarget true)
        (Variables|Default|SetLostSightTimer 0.0)
        (elif (Variables|Default|GetbHasTarget)
          (Variables|Default|SetLostSightTimer (+ (Variables|Default|GetLostSightTimer) DeltaSeconds))
          (if (>= (Variables|Default|GetLostSightTimer) (Variables|/Game/Data/BP_EnemyConfig.BP_EnemyConfig_C|GetLoseSightTime _enemyconfig))
            (Variables|Default|SetbHasTarget false))))
      (else
        (Variables|Default|SetPlayerTarget (Game|GetPlayerCharacter 0))
        (Variables|Default|SetTargetDistance (Math|Vector|VectorLength (- (Transformation|GetActorLocation (Variables|Default|GetPlayerTarget)) (Transformation|GetActorLocation _enemycharacter))))
        (Variables|Default|SetbSeesTarget (and (and (and (<= (Variables|Default|GetTargetDistance) (Math|Float|SelectFloat (Variables|/Game/Data/BP_EnemyConfig.BP_EnemyConfig_C|GetLoseSightRadius _enemyconfig) (Variables|/Game/Data/BP_EnemyConfig.BP_EnemyConfig_C|GetSightRadius _enemyconfig) (Variables|Default|GetbHasTarget))) (<= (Class|KismetMathLibrary|DegAcos (Math|Vector|DotProduct (Math|Vector|Normalize (- (Transformation|GetActorLocation (Variables|Default|GetPlayerTarget)) (Transformation|GetActorLocation _enemycharacter))) (Transformation|GetActorForwardVector _enemycharacter))) (Variables|/Game/Data/BP_EnemyConfig.BP_EnemyConfig_C|GetPeripheralVisionAngleDegrees _enemyconfig))) (Utilities|IsValid (Variables|Default|GetPlayerTarget))) (Controller|LineOfSightTo (Variables|Default|GetPlayerTarget) "0, 0, 0" false)))
        (if (Variables|Default|GetbSeesTarget)
          (Variables|Default|SetbHasTarget true)
          (Variables|Default|SetLostSightTimer 0.0)
          (elif (Variables|Default|GetbHasTarget)
            (Variables|Default|SetLostSightTimer (+ (Variables|Default|GetLostSightTimer) DeltaSeconds))
            (if (>= (Variables|Default|GetLostSightTimer) (Variables|/Game/Data/BP_EnemyConfig.BP_EnemyConfig_C|GetLoseSightTime _enemyconfig))
              (Variables|Default|SetbHasTarget false))))))))

(fn FacePlayerTarget
  (params (DeltaSeconds :type Float%20%28single-precision%29))
  (bind _playertarget (Variables|Default|GetPlayerTarget))
  (bind _enemycharacter (Variables|Default|GetEnemyCharacter))
  (if (and (Utilities|IsValid _playertarget) (Utilities|IsValid _enemycharacter))
    (Pawn|SetControlRotation (Math|Rotator|MakeRotator 0.0 0.0 (Class|KismetMathLibrary|FixedTurn (.Yaw (Math|Rotator|BreakRotator (Pawn|GetControlRotation :!class /Script/Engine.Controller))) (.Yaw (Math|Rotator|BreakRotator (Math|Rotator|MakeRotfromX (Math|Vector|Normalize (- (Transformation|GetActorLocation _playertarget) (Transformation|GetActorLocation _enemycharacter)))))) (* (Variables|/Game/Data/BP_EnemyConfig.BP_EnemyConfig_C|GetTurnSpeedDegrees (Variables|Default|GetEnemyConfig)) DeltaSeconds))))))

(fn EnterState
  (params (NewState :type E_EnemyAIState%20Enum :default "NewEnumerator0"))
  (Variables|Default|SetAIState NewState)
  (switch Utilities|FlowControl|Switch|SwitchonE_EnemyAIState NewState
    (:NewEnumerator0
      (AI|Navigation|StopMovement))
    (:NewEnumerator1
      (Variables|/Script/Engine.CharacterMovementComponent|SetMaxWalkSpeed (Variables|/Script/Engine.Character|GetCharacterMovement (Variables|Default|GetEnemyCharacter)) (Variables|/Game/Data/BP_EnemyConfig.BP_EnemyConfig_C|GetChaseSpeed (Variables|Default|GetEnemyConfig)))
      (Variables|Default|SetLastMoveRequestTime -1e+03))
    (:NewEnumerator2
      (AI|Navigation|StopMovement))))

(fn TryAttack
  (bind _playertarget (Variables|Default|GetPlayerTarget))
  (bind _enemyconfig (Variables|Default|GetEnemyConfig))
  (if (Utilities|IsValid _playertarget)
    (if (>= (- (Utilities|Time|GetGameTimeinSeconds) (Variables|Default|GetLastAttackTime)) (Variables|/Game/Data/BP_EnemyConfig.BP_EnemyConfig_C|GetAttackCooldown _enemyconfig))
      (bind _asbpi_damageable (Utilities|Casting|CastToBPI_Damageable _playertarget)
        (:then
          (Default|ApplyDamage _asbpi_damageable (Variables|/Game/Data/BP_EnemyConfig.BP_EnemyConfig_C|GetAttackDamage _enemyconfig)))
        (:CastFailed
          _))
      (Variables|Default|SetLastAttackTime (Utilities|Time|GetGameTimeinSeconds)))))